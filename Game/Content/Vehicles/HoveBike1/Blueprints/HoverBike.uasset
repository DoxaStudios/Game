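; Rideable hover bike that seats a ThirdPersonCharacter on its Seat socket and hands possession back on Interact.
; While the engine is on, Tick calls HoveringFunc, easing height above a downward trace, and input drives movement, yaw steering and mesh tilt.
; It also handles turbo, headlights, thruster particles, free-look and reverse camera, plus rider-gated inventory and debug widgets.
; OffFunc, a lower-height variant of the hover, is never called here.
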(event Custom|Attach
  (Class|SceneComponent|Attachto (Variables|/Script/Engine.Character|GetCapsuleComponent (Variables|Default|GetCharacter)) (Variables|Character|GetMesh) "Seat" "SnapToTarget" true))

(event Custom|Debug)

(event Custom|Inventory)

(event EventBeginPlay
  (Variables|Default|SetDefaultYaw (.Yaw (Class|KismetMathLibrary|BreakRot (Variables|/Script/Engine.SceneComponent|GetRelativeRotation (Variables|Default|GetSpringArm))))))

(event EventTick
  (params (DeltaSeconds :type Float%20%28single-precision%29))
  (if (Variables|Default|GetisEngineOn)
    (CallFunction|HoveringFunc DeltaSeconds)))

(event Input|ActionEvents|InputActionTacLook
  (bind _springarm (Variables|Default|GetSpringArm))
  (bind _relativerotation (Variables|/Script/Engine.SceneComponent|GetRelativeRotation _springarm))
  (bind (_pitch _yaw _roll) (Class|KismetMathLibrary|BreakRot _relativerotation))
  (:Pressed
    (Variables|Default|SetTacLook true))
  (:Released
    (Variables|Default|SetTacLook false)
    (Transformation|SetRelativeRotation _springarm (Class|KismetMathLibrary|MakeRot _pitch (Variables|Default|GetDefaultYaw) _roll) false)))

(event Input|ActionEvents|InputActionDebug
  (:Pressed
    (bind _asthird_person_character (Utilities|Casting|CastToThirdPersonCharacter (Variables|Default|GetCharacter)))
    (bind _returnvalue (Class|GameCharacter|EnableDisableKeys _asthird_person_character))
    (if _returnvalue
      (bind _returnvalue_2 (UserInterface|CreateWidget "/Game/UI/Blueprints/DebugUI/ItemDebug.ItemDebug_C"))
      (UserInterface|Viewport|AddtoViewport _returnvalue_2 0)
      (else
        (Default|End _returnvalue_2)))))

(event Input|ActionEvents|InputActionInventory
  (:Pressed
    (bind _asthird_person_character (Utilities|Casting|CastToThirdPersonCharacter (Variables|Default|GetCharacter)))
    (bind _returnvalue (Class|GameCharacter|EnableDisableKeys _asthird_person_character))
    (if _returnvalue
      (bind _returnvalue_2 (UserInterface|CreateWidget "/Game/UI/Blueprints/Inventory/w_Inventory.w_Inventory_C"))
      (UserInterface|Viewport|AddtoViewport _returnvalue_2 0)
      (else
        (Widget|RemovefromParent _returnvalue_2)))))

(event Input|ActionEvents|InputActionHeadlights
  (bind _spotlight (Variables|Default|GetSpotLight))
  (:Pressed
    (if (Variables|Default|GetisHeadlightsOn)
      (Rendering|Components|Light|SetIntensity _spotlight 0.0)
      (Variables|Default|SetisHeadlightsOn false)
      (else
        (Rendering|Components|Light|SetIntensity _spotlight (Variables|Default|GetHeadlightIntensity))
        (Variables|Default|SetisHeadlightsOn true)))))

(event Input|ActionEvents|InputActionInteract
  (bind _character (Variables|Default|GetCharacter))
  (:Pressed
    (Pawn|Possess (Game|GetPlayerController 0) _character)
    (Class|Actor|DetachRootComponentfromParent _character true)
    (bind _asthird_person_character (Utilities|Casting|CastToThirdPersonCharacter _character))
    (Variables|/Game/ThirdPerson/Blueprints/ThirdPersonCharacter.ThirdPersonCharacter_C|SetisSitting _asthird_person_character false)
    (Transformation|SetActorRotation _asthird_person_character)))

(event Input|ActionEvents|InputActionSprint
  (bind _charactermovement (Variables|Character|GetCharacterMovement))
  (:Pressed
    (Variables|/Script/Engine.CharacterMovementComponent|SetMaxFlySpeed _charactermovement (Variables|Default|GetTurbo%20Speed)))
  (:Released
    (Variables|/Script/Engine.CharacterMovementComponent|SetMaxFlySpeed _charactermovement (Variables|Default|GetNormal%20Speed))))

(event Input|AxisEvents|InputAxisMoveForward
  (params (AxisValue :type Float%20%28single-precision%29))
  (if (Variables|Default|GetisEngineOn)
    (Pawn|Input|AddMovementInput (Math|Vector|GetForwardVector (Class|KismetMathLibrary|MakeRot 0.0 (.Yaw (Class|KismetMathLibrary|BreakRot (Pawn|GetControlRotation :!class /Script/Engine.Pawn))) 0.0)) AxisValue false)))

(event Input|AxisEvents|InputAxisTurn
  (params (AxisValue :type Float%20%28single-precision%29))
  (bind _taclook (Variables|Default|GetTacLook))
  (bind _mesh (Variables|Character|GetMesh))
  (bind _relativerotation (Variables|/Script/Engine.SceneComponent|GetRelativeRotation _mesh))
  (bind (_pitch _yaw _roll) (Class|KismetMathLibrary|BreakRot _relativerotation))
  (if (Variables|Default|GetisEngineOn)
    (if _taclook
      (Transformation|AddRelativeRotation (Variables|Default|GetSpringArm) (Class|KismetMathLibrary|MakeRot 0.0 AxisValue 0.0) false :!label _label)
      (else
        (Pawn|Input|AddControllerYawInput (/ AxisValue 2.0))
        (Transformation|SetRelativeRotation (Variables|Character|GetMesh) (Class|KismetMathLibrary|MakeRot (* (+ (Math|Float|ClampAngle (- AxisValue 1.8e+02) 1e+01 -1e+01) 1.8e+02) -4.0) _yaw _roll) false)))
    (elif _taclook
      (goto _label))))

(event Input|AxisEvents|InputAxisMoveRight
  (params (AxisValue :type Float%20%28single-precision%29))
  (bind _mesh (Variables|Character|GetMesh))
  (bind _relativerotation (Variables|/Script/Engine.SceneComponent|GetRelativeRotation _mesh))
  (bind (_pitch _yaw _roll) (Class|KismetMathLibrary|BreakRot _relativerotation))
  (if (Variables|Default|GetisEngineOn)
    (Pawn|Input|AddControllerYawInput AxisValue)
    (Transformation|SetRelativeRotation (Variables|Character|GetMesh) (Class|KismetMathLibrary|MakeRot (* (+ (Math|Float|ClampAngle (- AxisValue 1.8e+02) 1e+01 -1e+01) 1.8e+02) -1e+01) _yaw _roll) false)))

(event Input|AxisEvents|InputAxisLookUp
  (params (AxisValue :type Float%20%28single-precision%29))
  (Transformation|AddRelativeRotation (Variables|Default|GetSpringArm) (Class|KismetMathLibrary|MakeRot AxisValue 0.0 0.0) false))

(event Input|KeyboardEvents|L
  (bind _particle2 (Variables|Default|Getparticle2))
  (:Pressed
    (if (Variables|Default|GetisEngineOn)
      (Variables|Default|SetisEngineOn false)
      (Development|SetHiddeninGame (Variables|Default|Getparticle1) true false)
      (else
        (Variables|Default|SetisEngineOn true)
        (Development|SetHiddeninGame _particle2 false false)
        (Components|Activation|Activate _particle2 true)))))

(event Input|MouseEvents|RightMouseButton
  (bind _springarm (Variables|Default|GetSpringArm))
  (:Pressed
    (Variables|/Script/Engine.SpringArmComponent|SetTargetArmLength _springarm -5e+02))
  (:Released
    (Variables|/Script/Engine.SpringArmComponent|SetTargetArmLength _springarm 5e+02)))

(fn ConstructionScript)

(fn HoveringFunc
  (params (DeltaTime :type Float%20%28single-precision%29))
  (bind _returnvalue (Transformation|GetActorLocation))
  (bind _returnvalue_2 (Transformation|GetActorLocation))
  (bind _capsulecomponent (Variables|Collision|GetCapsuleComponent))
  (bind _returnvalue_3 (Transformation|GetWorldLocation _capsulecomponent))
  (bind (_x _y _z) (Math|Vector|BreakVector _returnvalue))
  (bind (_x_2 _y_2 _z_2) (Math|Vector|BreakVector _returnvalue_2))
  (bind (_outhit _returnvalue_4) (Collision|LineTraceByChannel 0 _returnvalue_3 (- _returnvalue_3 "0, 0,200.000000") "TraceTypeQuery1" false 0 "None"))
  (if _returnvalue_4
    (Transformation|SetActorLocation (Math|Vector|MakeVector _x _y (Math|Interpolation|FInterpTo _z (+ (.Z (Math|Vector|BreakVector (.ImpactPoint (Collision|BreakHitResult _outhit)))) 1e+02) DeltaTime 5.0)) false)
    (else
      (Transformation|SetActorLocation (Math|Vector|MakeVector _x_2 _y_2 (Math|Interpolation|FInterpTo _z_2 (+ (.Z (Math|Vector|BreakVector (.TraceEnd (Collision|BreakHitResult _outhit)))) 1e+02) DeltaTime 5.0)) false))))

(fn OffFunc
  (params (Delta :type Float%20%28single-precision%29))
  (bind _returnvalue (Transformation|GetActorLocation))
  (bind _returnvalue_2 (Transformation|GetActorLocation))
  (bind _capsulecomponent (Variables|Collision|GetCapsuleComponent))
  (bind _returnvalue_3 (Transformation|GetWorldLocation _capsulecomponent))
  (bind (_x _y _z) (Math|Vector|BreakVector _returnvalue))
  (bind (_x_2 _y_2 _z_2) (Math|Vector|BreakVector _returnvalue_2))
  (bind (_outhit _returnvalue_4) (Collision|LineTraceByChannel 0 _returnvalue_3 (- _returnvalue_3 "0, 0,25.000000") "TraceTypeQuery1" false 0 "None"))
  (if _returnvalue_4
    (Transformation|SetActorLocation (Math|Vector|MakeVector _x_2 _y_2 (Math|Interpolation|FInterpTo _z_2 (+ (.Z (Math|Vector|BreakVector (.ImpactPoint (Collision|BreakHitResult _outhit)))) 25.0) Delta 1e+01)) false)
    (else
      (Transformation|SetActorLocation (Math|Vector|MakeVector _x _y (Math|Interpolation|FInterpTo _z (+ (.Z (Math|Vector|BreakVector (.TraceEnd (Collision|BreakHitResult _outhit)))) 25.0) Delta 1.0)) false))))